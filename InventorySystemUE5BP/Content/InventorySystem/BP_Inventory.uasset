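; Inventory component that stores item stacks as name and quantity entries and detects interactable actors in view.
; Tick, noted as every 0.1 seconds, sphere-traces from the player camera and prints each newly hit actor's interaction message.
; AddToInventory adds units singly to stacks below their DT_Items size limit, otherwise into empty slots, reporting any remainder.
; RemoveFromInventory is an empty stub, and Slot always returns index 0 for matches.
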(event EventTick
  (params (DeltaSeconds :type Float%20%28single-precision%29))
  (bind _returnvalue (Game|GetPlayerCameraManager 0))
  (bind _returnvalue_2 (Transformation|GetActorLocation _returnvalue))
  ;[1 1 1] Every 0.1 seconds , Trace a Sphere to see if an object is interactable ( Check Class Defaults to change tick strenght)
  (bind (_outhit _returnvalue_3) (Collision|SphereTraceByChannel _returnvalue_2 (+ _returnvalue_2 (* (Transformation|GetActorForwardVector _returnvalue) (Variables|Default|GetRange))) 2e+01 "TraceTypeQuery3" false (Utilities|Array|MakeArray (Components|GetOwner)) "Persistent"))
  (if _returnvalue_3
    (if (!= (.hitactor _outhit) (Variables|Default|GetHit%20Actor))
      (bind _output_get (Variables|Default|SetHit%20Actor (.hitactor _outhit)))
      (bind _itemname (Class|BPIInventory|InteractableActor(Message) _output_get))
      (Development|PrintText _itemname))))

(fn AddtoInventory
  (params (ItemName :type Name) (Quantity :type Integer))
  (Variables|Default|SetRemainingQuantity Quantity)
  (while (and (> (Variables|Default|GetRemainingQuantity) 0) (not (Variables|Default|GetFailed)))
    (bind (_index _foundslot) (CallFunction|Slot ItemName))
    (if _foundslot
      (CallFunction|AddtoLot _index 1)
      (Math|Integer|DecrementInt (Variables|Default|GetRemainingQuantity))
      (elif (.HasEmptySlot (CallFunction|AnyEmptySlotAvailable))
        (bind _success (CallFunction|CreateNewStack ItemName 1))
        (if _success
          (Math|Integer|DecrementInt (Variables|Default|GetRemainingQuantity))
          (else
            (Variables|Default|SetFailed true)))
        (else
          (Variables|Default|SetFailed true)))))
  (return (not (Variables|Default|GetFailed)) (Variables|Default|GetRemainingQuantity)))

(fn RemovefromInventory)

(fn Slot
  (params (ItemName :type Name))
  (for _array_element (Variables|Default|GetInventoryStructure)
    (if (== (.Name (Utilities|Struct|BreakBP_InventoryStructure _array_element)) ItemName)
      (if (< (.Quantity (Utilities|Struct|BreakBP_InventoryStructure _array_element)) (CallFunction|GetMaxStackSize ItemName))
        (return 0 true))))
  (return -1 false))

(fn GetMaxStackSize
  (params (ItemName :type Name))
  (bind _returnvalue (Utilities|GetDataTableRow "/Game/InventorySystem/DT_Items.DT_Items" ItemName)
    (:then
      (return (.LotSize (Utilities|Struct|BreakBP_ItemStructure _returnvalue))))
    (:RowNotFound
      (return -1))))

(fn AddtoLot
  (params (Index :type Integer) (Quantity :type Integer))
  (bind _inventorystructure (Variables|Default|GetInventoryStructure))
  (bind _output (Utilities|Array|Get(acopy) _inventorystructure Index))
  (Utilities|Array|SetArrayElem (Variables|Default|GetInventoryStructure) Index (Utilities|Struct|MakeBP_InventoryStructure (.name _output) (+ (.quantity _output) Quantity))))

(fn AnyEmptySlotAvailable
  (for (_array_element _array_index) (Variables|Default|GetInventoryStructure)
    (if (== (.Quantity (Utilities|Struct|BreakBP_InventoryStructure _array_element)) 0)
      (return true _array_index)))
  (return false -1))

(fn CreateNewStack
  (params (Item%20Name :type Name) (Quantity :type Integer))
  (bind (_hasemptyslot _emptyindex) (CallFunction|AnyEmptySlotAvailable))
  (if _hasemptyslot
    (Utilities|Array|SetArrayElem (Variables|Default|GetInventoryStructure) _emptyindex (Utilities|Struct|MakeBP_InventoryStructure Item%20Name Quantity))
    (return true)
    (else
      (return false))))

(fn InteractableActor
  (return ""))